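; Base enemy Blueprint that damages the player ship on contact and can be destroyed by damage.
; AnyDamage subtracts from Health, pushes it to the WB_PlayerEnemy widget in EnemyHealth, and destroys the actor at zero or below.
; Hit applies fixed damage to BP_Playership, using an Attacking flag and Delay as a cooldown.
; The flag is set before the cast, so hitting any other actor leaves it stuck on.
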(event `self.ReceiveAnyDamage`
  (params (Damage :type "Float (single-precision)") (DamageType :type "DamageType Object Reference") (InstigatedBy :type "Controller Object Reference") (DamageCauser :type "Actor Object Reference"))
  (set `self.Health` (- (`self.Health`) Damage))
  (`self.Update Health`)
  (if (<= (`self.Health`) 0.0)
    (`self.K2_DestroyActor`)))

(event `self.ReceiveHit`
  (params (MyComp :type "PrimitiveComponent Object Reference") (Other :type "Actor Object Reference") (OtherComp :type "PrimitiveComponent Object Reference") (bSelfMoved :type Boolean) (HitLocation :type "Vector Structure") (HitNormal :type "Vector Structure") (NormalImpulse :type "Vector Structure") (Hit :type "HitResult Structure (by ref)"))
  (if (not (`self.Attacking`))
    (set `self.Attacking` true)
    (bind _asbp_playership (cast `/Game/ShipAssets/BP_Playership` Other))
    (`GameplayStatics.ApplyDamage` _asbp_playership 10.0)
    (`KismetSystemLibrary.Delay` 1.0)
    (set `self.Attacking` false)))

(fn `Update Health`
  (bind _aswb_player_enemy (cast `/Game/ShipAssets/ShipUi/WB_PlayerEnemy` (`WidgetComponent.GetUserWidgetObject` (`self.Enemy Health`))))
  (set `/Game/ShipAssets/ShipUi/WB_PlayerEnemy.UIHealth` (`self.Health`) _aswb_player_enemy)
  (return))

(fn `UserConstructionScript`)