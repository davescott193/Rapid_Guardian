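; Player-controlled ship Character that sails forward constantly along its mesh's heading, with axis input steering yaw and a timed dash boosting speed.
; Right and left mouse buttons fire broadsides from tag-gathered spawn components, spawning projectiles and fire emitters under one shared cooldown.
; Damage updates a widget-component health bar, activates smoke at low health and opens MainMenu at zero.
; The PlayerMenuAction input applies damage to the ship itself.
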(event `Key|RightMouseButton`
  (params (Key :type "Key Structure"))
  (:`Pressed`
    (if (not (`self.Fire CoolDown`))
      (set `self.Fire CoolDown` true)
      (for _array_element (`self.RightProjectiles`)
        (bind (_returnvalue_location _returnvalue_rotation) (`KismetMathLibrary.BreakTransform` (`SceneComponent.K2_GetComponentToWorld` _array_element)))
        (bind _returnvalue (`|SpawnActorFromClass` "/Game/TopDown/Blueprints/BP_Projectile.BP_Projectile_C" (`KismetMathLibrary.MakeTransform` _returnvalue_location _returnvalue_rotation (`self.Spawn Transform Scale`)) "AlwaysSpawn" "OverrideRootScale" null null))
        (bind _returnvalue_2 (`GameplayStatics.SpawnEmitterAttached` "/Game/StarterContent/Particles/P_Fire.P_Fire" _array_element "None" (`self.K2_GetActorLocation` _returnvalue) (struct) (5.0 5.0 5.0) "KeepWorldPosition"))
        (`KismetArrayLibrary.Array_Add` (`self.Emmitter`) _returnvalue_2))
      (`KismetSystemLibrary.Delay` 2.0)
      (set `self.Fire CoolDown` false)
      (for _array_element_2 (`self.Emmitter`)
        (`/Engine/EditorBlueprintResources/StandardMacros.IsValid` _array_element_2
          (:`Is Valid`
            (`ActorComponent.K2_DestroyComponent` _array_element_2)))))))

(event `Key|LeftMouseButton`
  (params (Key :type "Key Structure"))
  (:`Pressed`
    (if (not (`self.Fire CoolDown`))
      (set `self.Fire CoolDown` true)
      (for _array_element (`self.LeftProjectiles`)
        (bind (_returnvalue_location _returnvalue_rotation) (`KismetMathLibrary.BreakTransform` (`SceneComponent.K2_GetComponentToWorld` _array_element)))
        (bind _returnvalue (`|SpawnActorFromClass` "/Game/TopDown/Blueprints/BP_Projectile.BP_Projectile_C" (`KismetMathLibrary.MakeTransform` _returnvalue_location _returnvalue_rotation (`self.Spawn Transform Scale`)) "AlwaysSpawn" "OverrideRootScale" null null))
        (bind _returnvalue_2 (`GameplayStatics.SpawnEmitterAttached` "/Game/StarterContent/Particles/P_Fire.P_Fire" _array_element "None" (`self.K2_GetActorLocation` _returnvalue) (struct) (5.0 5.0 5.0) "KeepWorldPosition"))
        (`KismetArrayLibrary.Array_Add` (`self.Emmitter`) _returnvalue_2))
      (`KismetSystemLibrary.Delay` 2.0)
      (set `self.Fire CoolDown` false)
      (for _array_element_2 (`self.Emmitter`)
        (`/Engine/EditorBlueprintResources/StandardMacros.IsValid` _array_element_2
          (:`Is Valid`
            (`ActorComponent.K2_DestroyComponent` _array_element_2)))))))

(event `self.ReceiveTick`
  (params (DeltaSeconds :type "Float (single-precision)"))
  (`self.AddMovementInput` (`KismetMathLibrary.GetForwardVector` (`SceneComponent.K2_GetComponentRotation` (`self.SM_Ship`))) 0.8))

(event `InputAxis|MoveRight-Left`
  (params (AxisValue :type "Float (single-precision)"))
  (bind _returnvalue (`KismetMathLibrary.MakeRotator` (.roll (`SceneComponent.K2_GetComponentRotation` (`self.SM_Ship`))) (.pitch (`SceneComponent.K2_GetComponentRotation` (`self.SM_Ship`))) (+ (.yaw (`SceneComponent.K2_GetComponentRotation` (`self.SM_Ship`))) (* 0.6 AxisValue))))
  (if (!= AxisValue 0.0)
    (`SceneComponent.K2_SetWorldRotation` (`self.SM_Ship`) _returnvalue false false)
    (`KismetSystemLibrary.PrintString` (`KismetStringLibrary.Conv_RotatorToString` _returnvalue))
    (`KismetSystemLibrary.PrintString` "Hello" true true (struct :`R` 1.0 :`G` 0.139431 :`A` 1.0))))

(event `self.ReceiveBeginPlay`
  (bind _returnvalue (`GameplayStatics.GetObjectClass` (`self.Projectile Spawn Left`)))
  ;[1 1 1] Start of the game Make sure health bar is the same value
  (`self.UpdateHealthBar`)
  (bind _asplayer_controller (cast `PlayerController` (`self.GetController`)))
  (bind _returnvalue_2 (pcsubsystem `EnhancedInputLocalPlayerSubsystem` _asplayer_controller))
  (`/Engine/EditorBlueprintResources/StandardMacros.IsValid` _returnvalue_2
    (:`Is Valid`
      (`EnhancedInputSubsystemInterface.AddMappingContext` _returnvalue_2 "/Game/ShipAssets/PlayerInputContex.PlayerInputContex" 0 (struct))
      (set `self.RightProjectiles` (`self.GetComponentsByTag` _returnvalue "Right"))
      (set `self.LeftProjectiles` (`self.GetComponentsByTag` _returnvalue "Left")))))

(event `EnhancedInput|/Game/ShipAssets/PlayerMenuAction`
  (params (ActionValue :type Boolean) (ElapsedSeconds :type "Float (double-precision)") (TriggeredSeconds :type "Float (double-precision)") (InputAction :type "InputAction Object Reference" :default "/Game/ShipAssets/PlayerMenuAction.PlayerMenuAction"))
  (:`Triggered`
    (`GameplayStatics.ApplyDamage` self 1.0)))

(event `self.ReceiveAnyDamage`
  (params (Damage :type "Float (single-precision)") (DamageType :type "DamageType Object Reference") (InstigatedBy :type "Controller Object Reference") (DamageCauser :type "Actor Object Reference"))
  ;[1 1 1] AnyDamageProccessing
  (set `self.Health` (- (`self.Health`) Damage))
  (`self.UpdateHealthBar`)
  (if (<= (`self.Health`) 0.0)
    (`KismetSystemLibrary.PrintString` "you lose")
    (`GameplayStatics.OpenLevel` "MainMenu")
    (else
      (`KismetSystemLibrary.PrintString` "You Took Damage")
      (if (<= (`self.Health`) 20.0)
        (`ActorComponent.Activate` (`self.Smoke1`) false)
        (if (<= (`self.Health`) 10.0)
          (`ActorComponent.Activate` (`self.Smoke`) false))))))

(event `EnhancedInput|/Game/ShipAssets/PlayerDash`
  (params (ActionValue :type Boolean) (ElapsedSeconds :type "Float (double-precision)") (TriggeredSeconds :type "Float (double-precision)") (InputAction :type "InputAction Object Reference" :default "/Game/ShipAssets/PlayerDash.PlayerDash"))
  (bind _charactermovement (`self.CharacterMovement`))
  (:`Triggered`
    (if (not (`self.IsDash`))
      (set `self.IsDash` true)
      (set `CharacterMovementComponent.MaxWalkSpeed` 1200.0 _charactermovement)
      (`KismetSystemLibrary.Delay` 1.0)
      (set `CharacterMovementComponent.MaxWalkSpeed` 600.0 _charactermovement)
      (set `self.IsDash` false))))

(fn `UpdateHealthBar`
  (bind _aswb_player_health_bar (cast `/Game/ShipAssets/ShipUi/WB_PlayerHealthBar` (`WidgetComponent.GetUserWidgetObject` (`self.WB_HealthBar`))))
  (set `/Game/ShipAssets/ShipUi/WB_PlayerHealthBar.UIHealth` (`self.Health`) _aswb_player_health_bar)
  (return))

(fn `UserConstructionScript`)